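; BP_Grenade is a thrown grenade actor that explodes half a second after Throw is called.
; Throw sets and activates ProjectileMovement while spinning the sphere to a random rotation during flight.
; On detonation it plays sound and particles, hides the sphere, sets a short lifespan, and sphere-traces for pawns.
; Each unique hit actor receives GrenadeHitMessage with the explosion location and damage.
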(event Custom|Throw
  (params (Velocity :type Vector))
  (bind _projectilemovement (Variables|Default|GetProjectileMovement))
  (bind _sphere (Variables|Default|GetSphere))
  (bind _sphere_2 (Variables|Default|GetSphere))
  (bind _returnvalue (Transformation|GetWorldLocation _sphere_2))
  (bind _returnvalue_2 (Transformation|GetWorldLocation _sphere))
  (Utilities|FlowControl|Sequence
    (:then_0
      (Variables|/Script/Engine.MovementComponent|SetVelocity _projectilemovement Velocity)
      (Components|Activation|Activate _projectilemovement false)
      (Utilities|FlowControl|Delay 0.5)
      (Audio|PlaySoundatLocation "/Game/NewFolder/Explosion.Explosion" _returnvalue_2 "0, 0, 0" 1.0 1.0 0.0 0 0 0)
      (Effects|SpawnEmitteratLocation "/Game/InfinityBladeEffects/Effects/FX_Mobile/Fire/combat/P_Buff_JumpDiveFire_02.P_Buff_JumpDiveFire_02" _returnvalue_2)
      (Development|SetHiddeninGame (Variables|Default|GetSphere) true false)
      (Actor|SetLifeSpan 3.0)
      (bind (_outhits _returnvalue_3) (Collision|MultiSphereTraceForObjects _returnvalue _returnvalue 5e+02 (Utilities|Array|MakeArray "ObjectTypeQuery3") false 0 "None"))
      (if _returnvalue_3
        (for _array_element _outhits
          (Utilities|Array|AddUnique (Variables|Default|Gethit%20actors) (.HitActor (Collision|BreakHitResult _array_element))))
        (for _array_element_2 (Variables|Default|Gethit%20actors)
          (Class|BPIMPCharacter|GrenadeHit(Message) _array_element_2 _returnvalue 2.0))))
    (:then_1
      (Components|MoveComponentTo (Variables|Default|GetSphere) "0, 0, 0" (Math|Random|RandomRotator false) false false 0.5 false))))

(event EventBeginPlay)

(event Collision|EventActorBeginOverlap
  (params (OtherActor :type Actor%20Object%20Reference)))

(event EventTick
  (params (DeltaSeconds :type Float%20%28single-precision%29)))

(fn ConstructionScript)